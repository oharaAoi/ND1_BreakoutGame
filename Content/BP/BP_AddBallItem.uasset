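; BP_AddBallItem is a falling pickup that adds a ball when the player touches it.
; Tick moves it down the Z axis at Speed, scaled by world delta time.
; Its Sphere overlap checks component tags: MissArea destroys the item, while Player first calls GenerateBall on the BP_GameManager found via GetActorOfClass, then destroys it.
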(event OnComponentBeginOverlap(Sphere)
  (params (OverlappedComponent :type Primitive%20Component%20Object%20Reference) (OtherActor :type Actor%20Object%20Reference) (OtherComp :type Primitive%20Component%20Object%20Reference) (OtherBodyIndex :type Integer) (bFromSweep :type Boolean) (SweepResult :type Hit%20Result%20Structure%20%28by%20ref%29))
  (if (Components|ComponentHasTag OtherComp "MissArea")
    (Actor|DestroyActor)
    (elif (Components|ComponentHasTag OtherComp "Player")
      (bind _returnvalue (Actor|GetActorOfClass "/Game/BP/BP_GameManager.BP_GameManager_C"))
      (Default|GenerateBall _returnvalue)
      (Actor|DestroyActor))))

(event EventBeginPlay)

(event Collision|EventActorBeginOverlap
  (params (OtherActor :type Actor%20Object%20Reference)))

(event EventTick
  (params (DeltaSeconds :type Float%20%28single-precision%29))
  (bind _returnvalue (Transformation|GetActorLocation))
  (Transformation|SetActorLocation (Math|Vector|MakeVector (.x _returnvalue) (.y _returnvalue) (- (.z _returnvalue) (* (Variables|Default|GetSpeed) (Utilities|Time|GetWorldDeltaSeconds)))) false false))

(fn ConstructionScript)