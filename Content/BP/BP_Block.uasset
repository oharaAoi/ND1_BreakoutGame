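; BP_Block is a breakable block that loses HP on each hit and is destroyed when it runs out.
; On BeginPlay it registers with BP_GameManager, and on destruction it reports the break and randomly spawns a BP_AddBallItem at its position.
; ReloadHp shows the current HP on a text render and tints a construction-script dynamic material from a ColorTable indexed by HP.
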(event EventBeginPlay
  (bind _returnvalue (Actor|GetActorOfClass "/Game/BP/BP_GameManager.BP_GameManager_C"))
  (Default|AddBlockNum _returnvalue)
  (CallFunction|ReloadHp))

(event Collision|EventActorBeginOverlap
  (params (OtherActor :type Actor%20Object%20Reference)))

(event EventTick
  (params (DeltaSeconds :type Float%20%28single-precision%29)))

(event Collision|EventHit
  (params (MyComp :type Primitive%20Component%20Object%20Reference) (Other :type Actor%20Object%20Reference) (OtherComp :type Primitive%20Component%20Object%20Reference) (bSelfMoved :type Boolean) (HitLocation :type Vector :default "0, 0, 0") (HitNormal :type Vector :default "0, 0, 0") (NormalImpulse :type Vector :default "0, 0, 0") (Hit :type Hit%20Result%20Structure%20%28by%20ref%29))
  (bind _result (Math|Integer|DecrementInt (Variables|Default|GetHp))
    (:%20%20
      (CallFunction|ReloadHp)
      (if (<= _result 0)
        (Actor|DestroyActor)
        (bind _returnvalue (Actor|GetActorOfClass "/Game/BP/BP_GameManager.BP_GameManager_C"))
        (Default|AddBrokenBlockNum _returnvalue)
        (if (Math|Random|RandomBoolwithWeight 0.5)
          (Game|SpawnActorfromClass "/Game/BP/BP_AddBallItem.BP_AddBallItem_C" (Transformation|GetActorTransform) "Undefined" "MultiplyWithRoot" 0 0))))))

(fn ConstructionScript
  (bind _returnvalue (Rendering|Material|CreateDynamicMaterialInstance (Variables|Default|GetCube) 0 0 "None" :!class /Script/Engine.PrimitiveComponent))
  (Variables|Default|SetMaterialInstance _returnvalue))

(fn ReloadHp
  (Rendering|Components|TextRender|SetText (Variables|Default|GetTextRender) (Utilities|Text|ToText(Integer) (Variables|Default|GetHp)))
  (if (Utilities|Array|IsValidIndex (Variables|Default|GetColorTable) (- (Variables|Default|GetHp) 1))
    (Rendering|Material|SetVectorParameterValue (Variables|Default|GetMaterialInstance) "BaseColor" (Math|Conversions|ToLinearColor(Color) (Utilities|Array|Get(acopy) (Variables|Default|GetColorTable) (- (Variables|Default|GetHp) 1))) :!class /Script/Engine.MaterialInstanceDynamic)))